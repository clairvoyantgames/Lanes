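; Player pawn for a two-player lane shooter; on BeginPlay it sets player ID and possesses a Hub by network authority.
; Keys 1–7 spawn a Shot in an empty lane or select an occupied one, updating HUD highlights.
; Then picking an adjacent, wrapping lane shifts that Shot, merging it with any occupant into a combined-health super shot.
; Enemy shot overlaps reduce health; spawned-shot lane and owner setup is disconnected.
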(event `self.ReceiveBeginPlay`
  (bind _returnvalue (`GameplayStatics.GetPlayerController` 0))
  ;[1 1 1] Set player ids
  (bind _outactors (`GameplayStatics.GetAllActorsOfClass` "Hub_C"))
  (`/Engine/EditorBlueprintResources/ActorMacros.Switch Has Authority`
    (:`Authority`
      (bind _ashub_c (cast `/Game/Blueprints/Hub` (`KismetArrayLibrary.Array_Get` _outactors)))
      (set `/Game/Blueprints/Hub.PlayerId` 0 _ashub_c)
      (`Controller.Possess` _returnvalue _ashub_c))
    (:`Remote`
      (bind _ashub_c_2 (cast `/Game/Blueprints/Hub` (`KismetArrayLibrary.Array_Get` _outactors 1)))
      (set `/Game/Blueprints/Hub.PlayerId` 1 _ashub_c_2)
      (`Controller.Possess` _returnvalue _ashub_c_2))))

(event `self.Box1.OnComponentBeginOverlap`
  (params (OtherActor :type "Actor Object Reference") (OtherComp :type "PrimitiveComponent Object Reference") (OtherBodyIndex :type Integer))
  ;[1 1 1] If shot hit player subtract health
  (bind _asshot_c (cast `/Game/Blueprints/Shot` OtherActor))
  (bind _player (`/Game/Blueprints/Shot.Player` _asshot_c))
  (if (and (!= (`/Game/Blueprints/Shot.Player` _asshot_c) null) (!= _player self))
    (set `self.playerHealth` (- (`self.playerHealth`) (`/Game/Blueprints/Shot.Health` _asshot_c)))
    ;[1 1 1] Setting gui icons back to normal
    (bind _returnvalue (`Controller.CastToPlayerController` (`self.GetController` _player)))
    (switch `int` (`/Game/Blueprints/Hub.previousSelection` _player)
      (:`Default`
        _)
      (:`0`
        (bind _returnvalue_2 (`PlayerController.GetHUD` _returnvalue))
        (message `/Game/Blueprints/isItClicked.is1Previous` _returnvalue_2 false))
      (:`1`
        (message `/Game/Blueprints/isItClicked.is2Previous` _returnvalue_2 false))
      (:`2`
        (message `/Game/Blueprints/isItClicked.is3Previous` _returnvalue_2 false))
      (:`3`
        (message `/Game/Blueprints/isItClicked.is4Previous` _returnvalue_2 false))
      (:`4`
        (message `/Game/Blueprints/isItClicked.is5Previous` _returnvalue_2 false))
      (:`5`
        (message `/Game/Blueprints/isItClicked.is6Previous` _returnvalue_2 false))
      (:`6`
        (message `/Game/Blueprints/isItClicked.is7Previous` _returnvalue_2 false)))
    (set `/Game/Blueprints/Hub.previousSelection` -1 _player)
    (set `/Game/Blueprints/Hub.ShotsFired` false _player)
    (`self.K2_DestroyActor` OtherActor)))

(event `Key|One`
  (bind _selectedshot (`self.SelectedShot`))
  (bind _newlaneshot (`self.newLaneShot`))
  (bind _pickedlane (`self.PickedLane`))
  (bind _lanes (`self.Lanes`))
  (bind _previousselection (`self.previousSelection`))
  (bind _returnvalue (`PlayerController.GetHUD` (`GameplayStatics.GetPlayerController` 0)))
  (bind _returnvalue_2 (`PlayerController.GetHUD` (`GameplayStatics.GetPlayerController` 0)))
  (bind _returnvalue_3 (`self.K2_GetActorLocation` (`self.SelectedShot`)))
  (bind _returnvalue_4 (`self.K2_GetActorLocation` (`self.newLaneShot`)))
  (bind _returnvalue_5 (`PlayerController.GetHUD` (`GameplayStatics.GetPlayerController` 0)))
  (bind _returnvalue_6 (- _previousselection 1))
  (bind _returnvalue_7 (+ _previousselection 1))
  (bind _returnvalue_8 (== _pickedlane (`KismetMathLibrary.SelectInt` (`KismetArrayLibrary.Array_LastIndex` _lanes) _returnvalue_6 (> 0 _returnvalue_6))))
  ;[1 1 1] Take input
  (:`Pressed`
    (message `/Game/Blueprints/isItClicked.isOneClicked` _returnvalue true)
    (if (not (`self.ShotsFired`))
      (set `self.PickedLane` 0)
      (set `self.DistanceMultiplier` -3.0)
      (set `self.ShotsFired` true :!label _label)
      ;[1 1 1] If there is a previous selection go to >
      (`/Engine/EditorBlueprintResources/StandardMacros.CompareInt` (`self.previousSelection`) -1
        (:`>`
          ;[1 1 1] Is Adjacent
          (if (or _returnvalue_8 (== _pickedlane (`KismetMathLibrary.SelectInt` _returnvalue_7 0 (< _returnvalue_7 (`KismetArrayLibrary.Array_Length` _lanes)))))
            ;[1 1 1] Handle Selection
            (set `self.Left` _returnvalue_8)
            (bind _outactors (`GameplayStatics.GetAllActorsOfClass` "/Game/Blueprints/Shot.Shot_C"))
            (for _array_element _outactors
              ;;[0.975 0 0.09497] Loop Through all the shots to see if a lane matches the previous location
              (bind _asshot_c (cast `/Game/Blueprints/Shot` _array_element))
              (if (== (`/Game/Blueprints/Shot.Lane` _asshot_c) (`self.previousSelection`))
                (set `self.SelectedShot` _asshot_c)))
            ;;[1 0.03055 0] Make sure the selected shot is from the previous lane
            (if (== (`/Game/Blueprints/Shot.Lane` (`self.SelectedShot`)) (`self.previousSelection`))
              ;;[1 1 1] Change the previous lane to be open(false) now
              (`KismetArrayLibrary.Array_Set` (`self.Lanes`) (`self.previousSelection`))
              ;;[1 1 1] Move actor over
              (`/Game/Blueprints/Shot.Shift Lane` (`self.SelectedShot`) (`self.Left`))
              ;;[1 1 1] If an actor is in new lane->true else
              (if (`KismetArrayLibrary.Array_Get` (`self.Lanes`) (`self.PickedLane`))
                ;;[1 0.01209 0] Loop through all shots to find the one in the new lane
                (bind _outactors_2 (`GameplayStatics.GetAllActorsOfClass` "/Game/Blueprints/Shot.Shot_C"))
                (for _array_element_2 _outactors_2
                  (bind _asshot_c_2 (cast `/Game/Blueprints/Shot` _array_element_2))
                  (if (== (`/Game/Blueprints/Shot.Lane` _asshot_c_2) (`self.PickedLane`))
                    (set `self.newLaneShot` _asshot_c_2)))
                ;;[1 0.03055 0] Make sure the selected shot is from the new lane
                (if (== (`/Game/Blueprints/Shot.Lane` (`self.newLaneShot`)) (`self.PickedLane`))
                  ;;[1 1 1] delay then destroy both actors
                  (`KismetSystemLibrary.Delay` 0.5)
                  (`self.K2_DestroyActor` _selectedshot)
                  (`self.K2_DestroyActor` _newlaneshot)
                  (`GameplayStatics.PlaySoundAtLocation` "/Game/Audio/Explosion01.Explosion01" _returnvalue_3)
                  (`GameplayStatics.PlaySoundAtLocation` null _returnvalue_4)
                  (bind _returnvalue_9 (`|SpawnActorFromClass` "/Game/Blueprints/Shot.Shot_C" (`KismetMathLibrary.Conv_VectorToTransform` (`KismetMathLibrary.VLerp` _returnvalue_3 _returnvalue_4 0.5)) true))
                  (set `/Game/Blueprints/Shot.Lane` (`self.PickedLane`) _returnvalue_9)
                  (set `/Game/Blueprints/Shot.Player` self _returnvalue_9)
                  (`/Game/Blueprints/Shot.makeASuper` _returnvalue_9 (+ (`/Game/Blueprints/Shot.Health` _selectedshot) (`/Game/Blueprints/Shot.Health` _newlaneshot)))
                  ;[1 1 1] Setting gui icons back to normal
                  (switch `int` (`self.previousSelection`) :!label _label_2
                    (:`0`
                      (message `/Game/Blueprints/isItClicked.is1Previous` _returnvalue_5 false))
                    (:`1`
                      (message `/Game/Blueprints/isItClicked.is2Previous` _returnvalue_5 false))
                    (:`2`
                      (message `/Game/Blueprints/isItClicked.is3Previous` _returnvalue_5 false))
                    (:`3`
                      (message `/Game/Blueprints/isItClicked.is4Previous` _returnvalue_5 false))
                    (:`4`
                      (message `/Game/Blueprints/isItClicked.is5Previous` _returnvalue_5 false))
                    (:`5`
                      (message `/Game/Blueprints/isItClicked.is6Previous` _returnvalue_5 false))
                    (:`6`
                      (message `/Game/Blueprints/isItClicked.is7Previous` _returnvalue_5 false)))
                  ;[1 1 1] Setting Previous back to default
                  (set `self.previousSelection` -1)
                  (set `self.ShotsFired` false))
                (else
                  (set `/Game/Blueprints/Shot.Lane` (`self.PickedLane`) (`self.SelectedShot`))
                  (`KismetArrayLibrary.Array_Set` (`self.Lanes`) (`self.PickedLane`) true)
                  (goto _label_2)))
              (else
                (goto _label_2)))
            (else
              (goto _label_2))))
        (:`==`
          ;[1 1 1] is the picked lane filled
          (if (`KismetArrayLibrary.Array_Get` (`self.Lanes`) (`self.PickedLane`))
            ;[1 1 1] Setting Previous Selection
            (set `self.ShotsFired` false)
            (set `self.previousSelection` (`self.PickedLane`))
            ;[1 1 1] Calling gui to change color of icons to white
            (switch `int` (`self.PickedLane`)
              (:`0`
                (message `/Game/Blueprints/isItClicked.is1Previous` _returnvalue_2 true))
              (:`1`
                (message `/Game/Blueprints/isItClicked.is2Previous` _returnvalue_2 true))
              (:`2`
                (message `/Game/Blueprints/isItClicked.is3Previous` _returnvalue_2 true))
              (:`3`
                (message `/Game/Blueprints/isItClicked.is4Previous` _returnvalue_2 true))
              (:`4`
                (message `/Game/Blueprints/isItClicked.is5Previous` _returnvalue_2 true))
              (:`5`
                (message `/Game/Blueprints/isItClicked.is6Previous` _returnvalue_2 true))
              (:`6`
                (message `/Game/Blueprints/isItClicked.is7Previous` _returnvalue_2 true)))
            (else
              (set `self.Selected` -1)
              (`self.Shot` (`KismetMathLibrary.MakeTransform` (`KismetMathLibrary.MakeVector` (.x (.location (`self.GetTransform`))) (+ (* 100.0 (`self.DistanceMultiplier`)) (.y (.location (`self.GetTransform`)))) (.z (.location (`self.GetTransform`)))) (.rotation (`self.GetTransform`))) (`self.PlayerId`))))))))
  (:`Released`
    (message `/Game/Blueprints/isItClicked.isOneClicked` _returnvalue false)))

(event `Key|Two`
  (bind _returnvalue (`PlayerController.GetHUD` (`GameplayStatics.GetPlayerController` 0)))
  ;[1 1 1] Take input
  (:`Pressed`
    (message `/Game/Blueprints/isItClicked.is2Clicked` _returnvalue true)
    (if (not (`self.ShotsFired`))
      (set `self.PickedLane` 1)
      (set `self.DistanceMultiplier` -2.0)
      (goto _label)))
  (:`Released`
    (message `/Game/Blueprints/isItClicked.is2Clicked` _returnvalue false)))

(event `Key|Three`
  (bind _returnvalue (`PlayerController.GetHUD` (`GameplayStatics.GetPlayerController` 0)))
  ;[1 1 1] Take input
  (:`Pressed`
    (message `/Game/Blueprints/isItClicked.is3Clicked` _returnvalue true)
    (if (not (`self.ShotsFired`))
      (set `self.PickedLane` 2)
      (set `self.DistanceMultiplier` -1.0)
      (goto _label)))
  (:`Released`
    (message `/Game/Blueprints/isItClicked.is3Clicked` _returnvalue false)))

(event `Key|Four`
  (bind _returnvalue (`PlayerController.GetHUD` (`GameplayStatics.GetPlayerController` 0)))
  ;[1 1 1] Take input
  (:`Pressed`
    (message `/Game/Blueprints/isItClicked.is4Clicked` _returnvalue true)
    (if (not (`self.ShotsFired`))
      (set `self.PickedLane` 3)
      (set `self.DistanceMultiplier` 0.0)
      (goto _label)))
  (:`Released`
    (message `/Game/Blueprints/isItClicked.is4Clicked` _returnvalue false)))

(event `Key|Five`
  (bind _returnvalue (`PlayerController.GetHUD` (`GameplayStatics.GetPlayerController` 0)))
  ;[1 1 1] Take input
  (:`Pressed`
    (message `/Game/Blueprints/isItClicked.is5Clicked` _returnvalue true)
    (if (not (`self.ShotsFired`))
      (set `self.PickedLane` 4)
      (set `self.DistanceMultiplier` 1.0)
      (goto _label)))
  (:`Released`
    (message `/Game/Blueprints/isItClicked.is5Clicked` _returnvalue false)))

(event `Key|Six`
  (bind _returnvalue (`PlayerController.GetHUD` (`GameplayStatics.GetPlayerController` 0)))
  ;[1 1 1] Take input
  (:`Pressed`
    (message `/Game/Blueprints/isItClicked.is6Clicked` _returnvalue true)
    (if (not (`self.ShotsFired`))
      (set `self.PickedLane` 5)
      (set `self.DistanceMultiplier` 2.0)
      (goto _label)))
  (:`Released`
    (message `/Game/Blueprints/isItClicked.is6Clicked` _returnvalue false)))

(event `Shot`
  (params (Location :type "Object.Transform Structure") (PlayerId :type Integer))
  ;[1 1 1] Shot Spawn
  (bind _returnvalue (`|SpawnActorFromClass` "/Game/Blueprints/Shot.Shot_C" Location)))

(event `Key|Seven`
  (bind _returnvalue (`PlayerController.GetHUD` (`GameplayStatics.GetPlayerController` 0)))
  ;[1 1 1] Take input
  (:`Pressed`
    (message `/Game/Blueprints/isItClicked.is7Clicked` _returnvalue true)
    (if (not (`self.ShotsFired`))
      (set `self.PickedLane` 6)
      (set `self.DistanceMultiplier` 3.0)
      (goto _label)))
  (:`Released`
    (message `/Game/Blueprints/isItClicked.is7Clicked` _returnvalue false)))

(fn `UserConstructionScript`)