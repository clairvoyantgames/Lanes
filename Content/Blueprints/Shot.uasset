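; Shot is a player-owned projectile that travels in a lane and is destroyed when it overlaps another player's Shot.
; Tick advances it along world X by Speed, while ShiftLane slides it sideways one lane width and clears the owner's ShotsFired flag.
; On collision it resets the owner's lane entry and selection state, restores the previous HUD icon, then destroys itself.
; MakeASuper sets its Health.
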(event `self.ReceiveActorBeginOverlap`
  (params (OtherActor :type "Actor Object Reference"))
  (bind _player (`self.Player`))
  (bind _player_2 (`self.Player`))
  ;[1 1 1] Destroy Colliding Shot
  (bind _asshot_c (cast `/Game/Blueprints/Shot` OtherActor))
  (if (!= (`/Game/Blueprints/Shot.Player` _asshot_c) _player)
    (`KismetArrayLibrary.Array_Set` (`/Game/Blueprints/Hub.Lanes` _player) (`self.Lane`))
    (set `/Game/Blueprints/Hub.ShotsFired` false _player_2)
    (set `/Game/Blueprints/Hub.Selected` -1 _player_2)
    ;[1 1 1] Setting gui icons back to normal
    (bind _returnvalue (`Controller.CastToPlayerController` (`Pawn.GetController` (`self.Player`))))
    (switch `int` (`/Game/Blueprints/Hub.previousSelection` (`self.Player`))
      (:`0`
        (bind _returnvalue_2 (`PlayerController.GetHUD` _returnvalue))
        (message `/Game/Blueprints/isItClicked.is1Previous` _returnvalue_2 false))
      (:`1`
        (message `/Game/Blueprints/isItClicked.is2Previous` _returnvalue_2 false))
      (:`2`
        (message `/Game/Blueprints/isItClicked.is3Previous` _returnvalue_2 false))
      (:`3`
        (message `/Game/Blueprints/isItClicked.is4Previous` _returnvalue_2 false))
      (:`4`
        (message `/Game/Blueprints/isItClicked.is5Previous` _returnvalue_2 false))
      (:`5`
        (message `/Game/Blueprints/isItClicked.is6Previous` _returnvalue_2 false))
      (:`6`
        (message `/Game/Blueprints/isItClicked.is7Previous` _returnvalue_2 false)))
    (set `/Game/Blueprints/Hub.previousSelection` -1 (`self.Player`))
    (`self.K2_DestroyActor` self)))

(event `self.ReceiveTick`
  (params (DeltaSeconds :type "Float (single-precision)"))
  ;[1 1 1] Constant Force
  (`self.K2_SetActorLocation` (`KismetMathLibrary.MakeVector` (+ (.x (`self.K2_GetActorLocation`)) (* (`GameplayStatics.GetWorldDeltaSeconds`) (`self.Speed`))) (.y (`self.K2_GetActorLocation`)) (.z (`self.K2_GetActorLocation`)))))

(event `Shift Lane`
  (params (Left :type Boolean))
  (bind _x (.x (`self.K2_GetActorLocation`)))
  (bind _y (.y (`self.K2_GetActorLocation`)))
  (bind _z (.z (`self.K2_GetActorLocation`)))
  ;[1 1 1] Shift
  (if Left
    (set `self.ShiftLocation` (`KismetMathLibrary.MakeVector` _x (- _y 100.0) _z))
    (else
      (set `self.ShiftLocation` (`KismetMathLibrary.MakeVector` _x (+ _y 100.0) _z))))
  (`KismetSystemLibrary.MoveComponentTo` (`self.K2_GetRootComponent`) (`self.ShiftLocation`))
  (set `/Game/Blueprints/Hub.ShotsFired` false (`self.Player`)))

(fn `makeASuper`
  (params (Health :type Integer))
  (set `self.Health` Health))

(fn `UserConstructionScript`)