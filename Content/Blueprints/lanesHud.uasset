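; HUD Blueprint that draws a row of seven round lane buttons along the lower screen on every DrawHUD.
; Flags from per-lane Previous and Clicked events pick grey, beige or blue textures.
; For lanes flagged in the player's Hub pawn, it searches all Shot actors each draw and prints matching shots' Health.
; The sixth button matches Lane 50 rather than 5, and only the first checks health when grey.
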(event `self.is1Previous`
  (params (NewParam :type Boolean)))

(event `self.isOneClicked`
  (params (NewParam :type Boolean)))

(event `self.is2Previous`
  (params (NewParam :type Boolean)))

(event `self.is2Clicked`
  (params (NewParam :type Boolean)))

(event `self.is3Previous`
  (params (NewParam :type Boolean)))

(event `self.is3Clicked`
  (params (NewParam :type Boolean)))

(event `self.is4Previous`
  (params (NewParam :type Boolean)))

(event `self.ReceiveDrawHUD`
  (params (SizeX :type Integer) (SizeY :type Integer))
  (bind _returnvalue (* (`KismetMathLibrary.Conv_IntToDouble` (`self.ScreenY`)) 0.8))
  (bind _returnvalue_2 (* (`KismetMathLibrary.Conv_IntToDouble` (`self.ScreenX`)) 0.63))
  (bind _returnvalue_3 (* (`KismetMathLibrary.Conv_IntToDouble` (`self.ScreenX`)) 0.27))
  (bind _returnvalue_4 (* (`KismetMathLibrary.Conv_IntToDouble` (`self.ScreenY`)) 0.8))
  (bind _returnvalue_5 (* (`KismetMathLibrary.Conv_IntToDouble` (`self.ScreenX`)) 0.33))
  (bind _returnvalue_6 (* (`KismetMathLibrary.Conv_IntToDouble` (`self.ScreenY`)) 0.8))
  (bind _returnvalue_7 (* (`KismetMathLibrary.Conv_IntToDouble` (`self.ScreenX`)) 0.39))
  (bind _returnvalue_8 (* (`KismetMathLibrary.Conv_IntToDouble` (`self.ScreenY`)) 0.8))
  (bind _returnvalue_9 (* (`KismetMathLibrary.Conv_IntToDouble` (`self.ScreenX`)) 0.45))
  (bind _returnvalue_10 (* (`KismetMathLibrary.Conv_IntToDouble` (`self.ScreenY`)) 0.8))
  (bind _returnvalue_11 (* (`KismetMathLibrary.Conv_IntToDouble` (`self.ScreenX`)) 0.51))
  (bind _returnvalue_12 (* (`KismetMathLibrary.Conv_IntToDouble` (`self.ScreenY`)) 0.8))
  (bind _returnvalue_13 (* (`KismetMathLibrary.Conv_IntToDouble` (`self.ScreenX`)) 0.57))
  (bind _returnvalue_14 (* (`KismetMathLibrary.Conv_IntToDouble` (`self.ScreenY`)) 0.8))
  (set `self.ScreenX` SizeX)
  (set `self.ScreenY` SizeY)
  (`|ExecutionSequence`
    (:`then_0`
      (if (stale `self.is1Previous` NewParam)
        (`self.DrawTextureSimple` "/Game/images/buttonRound_grey.buttonRound_grey" _returnvalue_3 _returnvalue_4)
        (elif (stale `self.isOneClicked` NewParam)
          (`self.DrawTextureSimple` "/Game/images/buttonRound_beige.buttonRound_beige" _returnvalue_3 _returnvalue_4)
          (else
            (`self.DrawTextureSimple` "/Game/images/buttonRound_blue.buttonRound_blue" _returnvalue_3 _returnvalue_4))))
      (bind _ashub_c (cast `/Game/Blueprints/Hub` (`GameplayStatics.GetPlayerPawn` 0)))
      (if (`KismetArrayLibrary.Array_Get` (`/Game/Blueprints/Hub.Lanes` _ashub_c))
        (bind _outactors (`GameplayStatics.GetAllActorsOfClass` "/Game/Blueprints/Shot.Shot_C"))
        (for _array_element _outactors
          (bind _asshot_c (cast `/Game/Blueprints/Shot` _array_element))
          (if (== (`/Game/Blueprints/Shot.Lane` _asshot_c) 0)
            (`self.DrawText` (`KismetStringLibrary.Conv_IntToString` (`/Game/Blueprints/Shot.Health` _asshot_c)) (struct :`G` 0.070531 :`B` 1.0 :`A` 1.0) 0.0 0.0 null 5.0)))))
    (:`then_1`
      (if (stale `self.is2Previous` NewParam)
        (`self.DrawTextureSimple` "/Game/images/buttonRound_grey.buttonRound_grey" _returnvalue_5 _returnvalue_6)
        (else
          (if (stale `self.is2Clicked` NewParam)
            (`self.DrawTextureSimple` "/Game/images/buttonRound_beige.buttonRound_beige" _returnvalue_5 _returnvalue_6)
            (else
              (`self.DrawTextureSimple` "/Game/images/buttonRound_blue.buttonRound_blue" _returnvalue_5 _returnvalue_6)))
          (bind _ashub_c_2 (cast `/Game/Blueprints/Hub` (`GameplayStatics.GetPlayerPawn` 0)))
          (if (`KismetArrayLibrary.Array_Get` (`/Game/Blueprints/Hub.Lanes` _ashub_c_2) 1)
            (bind _outactors_2 (`GameplayStatics.GetAllActorsOfClass` "/Game/Blueprints/Shot.Shot_C"))
            (for _array_element_2 _outactors_2
              (bind _asshot_c_2 (cast `/Game/Blueprints/Shot` _array_element_2))
              (if (== (`/Game/Blueprints/Shot.Lane` _asshot_c_2) 1)
                (`self.DrawText` (`KismetStringLibrary.Conv_IntToString` (`/Game/Blueprints/Shot.Health` _asshot_c_2)) (struct :`G` 0.070531 :`B` 1.0 :`A` 1.0) 0.0 0.0 null 5.0)))))))
    (:`then_2`
      (if (stale `self.is3Previous` NewParam)
        (`self.DrawTextureSimple` "/Game/images/buttonRound_grey.buttonRound_grey" _returnvalue_7 _returnvalue_8)
        (else
          (if (stale `self.is3Clicked` NewParam)
            (`self.DrawTextureSimple` "/Game/images/buttonRound_beige.buttonRound_beige" _returnvalue_7 _returnvalue_8)
            (else
              (`self.DrawTextureSimple` "/Game/images/buttonRound_blue.buttonRound_blue" _returnvalue_7 _returnvalue_8)))
          (bind _ashub_c_3 (cast `/Game/Blueprints/Hub` (`GameplayStatics.GetPlayerPawn` 0)))
          (if (`KismetArrayLibrary.Array_Get` (`/Game/Blueprints/Hub.Lanes` _ashub_c_3) 2)
            (bind _outactors_3 (`GameplayStatics.GetAllActorsOfClass` "/Game/Blueprints/Shot.Shot_C"))
            (for _array_element_3 _outactors_3
              (bind _asshot_c_3 (cast `/Game/Blueprints/Shot` _array_element_3))
              (if (== (`/Game/Blueprints/Shot.Lane` _asshot_c_3) 2)
                (`self.DrawText` (`KismetStringLibrary.Conv_IntToString` (`/Game/Blueprints/Shot.Health` _asshot_c_3)) (struct :`G` 0.070531 :`B` 1.0 :`A` 1.0) 0.0 0.0 null 5.0)))))))
    (:`then_3`
      (if (stale `self.is4Previous` NewParam)
        (`self.DrawTextureSimple` "/Game/images/buttonRound_grey.buttonRound_grey" _returnvalue_9 _returnvalue_10)
        (else
          (if (stale `self.is4Clicked` NewParam)
            (`self.DrawTextureSimple` "/Game/images/buttonRound_beige.buttonRound_beige" _returnvalue_9 _returnvalue_10)
            (else
              (`self.DrawTextureSimple` "/Game/images/buttonRound_blue.buttonRound_blue" _returnvalue_9 _returnvalue_10)))
          (bind _ashub_c_4 (cast `/Game/Blueprints/Hub` (`GameplayStatics.GetPlayerPawn` 0)))
          (if (`KismetArrayLibrary.Array_Get` (`/Game/Blueprints/Hub.Lanes` _ashub_c_4) 3)
            (bind _outactors_4 (`GameplayStatics.GetAllActorsOfClass` "/Game/Blueprints/Shot.Shot_C"))
            (for _array_element_4 _outactors_4
              (bind _asshot_c_4 (cast `/Game/Blueprints/Shot` _array_element_4))
              (if (== (`/Game/Blueprints/Shot.Lane` _asshot_c_4) 3)
                (`self.DrawText` (`KismetStringLibrary.Conv_IntToString` (`/Game/Blueprints/Shot.Health` _asshot_c_4)) (struct :`G` 0.070531 :`B` 1.0 :`A` 1.0) 0.0 0.0 null 5.0)))))))
    (:`then_4`
      (if (stale `self.is5Previous` NewParam)
        (`self.DrawTextureSimple` "/Game/images/buttonRound_grey.buttonRound_grey" _returnvalue_11 _returnvalue_12)
        (else
          (if (stale `self.is5Clicked` NewParam)
            (`self.DrawTextureSimple` "/Game/images/buttonRound_beige.buttonRound_beige" _returnvalue_11 _returnvalue_12)
            (else
              (`self.DrawTextureSimple` "/Game/images/buttonRound_blue.buttonRound_blue" _returnvalue_11 _returnvalue_12)))
          (bind _ashub_c_5 (cast `/Game/Blueprints/Hub` (`GameplayStatics.GetPlayerPawn` 0)))
          (if (`KismetArrayLibrary.Array_Get` (`/Game/Blueprints/Hub.Lanes` _ashub_c_5) 4)
            (bind _outactors_5 (`GameplayStatics.GetAllActorsOfClass` "/Game/Blueprints/Shot.Shot_C"))
            (for _array_element_5 _outactors_5
              (bind _asshot_c_5 (cast `/Game/Blueprints/Shot` _array_element_5))
              (if (== (`/Game/Blueprints/Shot.Lane` _asshot_c_5) 4)
                (`self.DrawText` (`KismetStringLibrary.Conv_IntToString` (`/Game/Blueprints/Shot.Health` _asshot_c_5)) (struct :`G` 0.070531 :`B` 1.0 :`A` 1.0) 0.0 0.0 null 5.0)))))))
    (:`then_5`
      (if (stale `self.is6Previous` NewParam)
        (`self.DrawTextureSimple` "/Game/images/buttonRound_grey.buttonRound_grey" _returnvalue_13 _returnvalue_14)
        (else
          (if (stale `self.is6Clicked` NewParam)
            (`self.DrawTextureSimple` "/Game/images/buttonRound_beige.buttonRound_beige" _returnvalue_13 _returnvalue_14)
            (else
              (`self.DrawTextureSimple` "/Game/images/buttonRound_blue.buttonRound_blue" _returnvalue_13 _returnvalue_14)))
          (bind _ashub_c_6 (cast `/Game/Blueprints/Hub` (`GameplayStatics.GetPlayerPawn` 0)))
          (if (`KismetArrayLibrary.Array_Get` (`/Game/Blueprints/Hub.Lanes` _ashub_c_6) 5)
            (bind _outactors_6 (`GameplayStatics.GetAllActorsOfClass` "/Game/Blueprints/Shot.Shot_C"))
            (for _array_element_6 _outactors_6
              (bind _asshot_c_6 (cast `/Game/Blueprints/Shot` _array_element_6))
              (if (== (`/Game/Blueprints/Shot.Lane` _asshot_c_6) 50)
                (`self.DrawText` (`KismetStringLibrary.Conv_IntToString` (`/Game/Blueprints/Shot.Health` _asshot_c_6)) (struct :`G` 0.070531 :`B` 1.0 :`A` 1.0) 0.0 0.0 null 5.0)))))))
    (:`then_6`
      (if (stale `self.is7Previous` NewParam)
        (`self.DrawTextureSimple` "/Game/images/buttonRound_grey.buttonRound_grey" _returnvalue_2 _returnvalue)
        (else
          (if (stale `self.is7Clicked` NewParam)
            (`self.DrawTextureSimple` "/Game/images/buttonRound_beige.buttonRound_beige" _returnvalue_2 _returnvalue)
            (else
              (`self.DrawTextureSimple` "/Game/images/buttonRound_blue.buttonRound_blue" _returnvalue_2 _returnvalue)))
          (bind _ashub_c_7 (cast `/Game/Blueprints/Hub` (`GameplayStatics.GetPlayerPawn` 0)))
          (if (`KismetArrayLibrary.Array_Get` (`/Game/Blueprints/Hub.Lanes` _ashub_c_7) 6)
            (bind _outactors_7 (`GameplayStatics.GetAllActorsOfClass` "/Game/Blueprints/Shot.Shot_C"))
            (for _array_element_7 _outactors_7
              (bind _asshot_c_7 (cast `/Game/Blueprints/Shot` _array_element_7))
              (if (== (`/Game/Blueprints/Shot.Lane` _asshot_c_7) 6)
                (`self.DrawText` (`KismetStringLibrary.Conv_IntToString` (`/Game/Blueprints/Shot.Health` _asshot_c_7)) (struct :`G` 0.070531 :`B` 1.0 :`A` 1.0) 0.0 0.0 null 5.0)))))))))

(event `self.is4Clicked`
  (params (NewParam :type Boolean)))

(event `self.is5Previous`
  (params (NewParam :type Boolean)))

(event `self.is5Clicked`
  (params (NewParam :type Boolean)))

(event `self.is6Previous`
  (params (NewParam :type Boolean)))

(event `self.is6Clicked`
  (params (NewParam :type Boolean)))

(event `self.is7Previous`
  (params (NewParam :type Boolean)))

(event `self.is7Clicked`
  (params (NewParam :type Boolean)))

(fn `UserConstructionScript`)