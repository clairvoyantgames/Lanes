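; Player pawn for a two-player networked lane duel, placing the non-local player opposite the other and assigning IDs by authority.
; Keys 1-3, mirrored per player, fire a Shot into an empty lane or select an occupied one.
; Picking an adjacent lane shifts the selected shot, merging with any shot there into a super shot with summed damage.
; Enemy shots overlapping Box1 reduce Health and free the shooter's lane.
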(event `self.ReceiveBeginPlay`
  ;[1 1 1] Moving 2nd player
  (`/Engine/EditorBlueprintResources/ActorMacros.Switch Has Authority`
    (:`Authority`
      (set `self.PlayerId` 0))
    (:`Remote`
      (set `self.PlayerId` 1))))

(event `destroyboth`
  (params (firstone :type "/Game/Blueprints/shot Object Reference") (secondOne :type "/Game/Blueprints/shot Object Reference") (newHealth :type Integer) (transform :type "Object.Transform Structure") (Lane :type Integer) (playerObject :type "Object Object Reference"))
  (`self.K2_DestroyActor` firstone)
  (`self.K2_DestroyActor` secondOne)
  (bind _returnvalue (`|SpawnActorFromClass` "/Game/Blueprints/shot.shot_C" transform true))
  (set `/Game/Blueprints/shot.Player` 0 _returnvalue)
  (set `/Game/Blueprints/shot.Lane` Lane _returnvalue)
  (set `/Game/Blueprints/shot.playerObject` playerObject _returnvalue)
  (`/Game/Blueprints/shot.makeASuper` _returnvalue newHealth))

(event `self.ReceivePossessed`
  (params (NewController :type "Controller Object Reference"))
  (bind _returnvalue (`Controller.GetControlledPawn` NewController))
  ;[1 1 1] Moving 2nd player
  (if (not (`Controller.IsLocalPlayerController` NewController))
    (`self.K2_TeleportTo` (`KismetMathLibrary.MakeVector` (+ (.x (`self.K2_GetActorLocation` _returnvalue)) 1000.0) (.y (`self.K2_GetActorLocation` _returnvalue)) (.z (`self.K2_GetActorLocation` _returnvalue))) (`KismetMathLibrary.MakeRot` (.pitch (`self.K2_GetActorRotation` _returnvalue)) (+ (.yaw (`self.K2_GetActorRotation` _returnvalue)) 180.0) (.roll (`self.K2_GetActorRotation` _returnvalue))))))

(event `ShiftLaneOfShot`
  (params (theShot :type "Object Object Reference") (left :type Boolean) (playerObject :type "Object Object Reference"))
  (bind _asshot_c (cast `/Game/Blueprints/shot` theShot))
  (`/Game/Blueprints/shot.Shift Lane` _asshot_c left))

(event `Key|One`
  (bind _selectedshot (`self.SelectedShot`))
  (bind _newlaneshot (`self.newLaneShot`))
  (bind _selectedshot_2 (`self.SelectedShot`))
  (bind _lanes (`self.Lanes`))
  (bind _pickedlane (`self.pickedLane`))
  (bind _previousselection (`self.previousSelection`))
  (bind _returnvalue (== (`self.PlayerId`) 0))
  (bind _returnvalue_2 (- _previousselection 1))
  (bind _returnvalue_3 (+ _previousselection 1))
  (bind _returnvalue_4 (== _pickedlane (`KismetMathLibrary.SelectInt` (`KismetArrayLibrary.Array_LastIndex` _lanes) _returnvalue_2 (> 0 _returnvalue_2))))
  (:`Pressed`
    (set `self.pickedLane` (`KismetMathLibrary.SelectInt` 0 2 _returnvalue))
    (set `self.distanceMultiplier` (`KismetMathLibrary.SelectFloat` -1.0 1.0 _returnvalue))
    (`/Engine/EditorBlueprintResources/StandardMacros.CompareInt` (`self.previousSelection`) -1 :!label _label
      (:`>`
        ;[1 1 1] Is Adjacent
        (if (or _returnvalue_4 (== _pickedlane (`KismetMathLibrary.SelectInt` _returnvalue_3 0 (< _returnvalue_3 (`KismetArrayLibrary.Array_Length` _lanes)))))
          (set `self.Left` _returnvalue_4)
          (bind _outactors (`GameplayStatics.GetAllActorsOfClass` "/Game/Blueprints/shot.shot_C"))
          (for _array_element _outactors
            (bind _asshot_c (cast `/Game/Blueprints/shot` _array_element))
            (if (== (`/Game/Blueprints/shot.playerObject` _asshot_c) self)
              (if (== (`/Game/Blueprints/shot.Lane` _asshot_c) (`self.previousSelection`))
                (set `self.SelectedShot` _asshot_c))))
          (if (not (== _selectedshot_2 null))
            ;[1 0.03055 0] Make sure the selected shot is from the previous lane
            (if (== (`/Game/Blueprints/shot.Lane` _selectedshot_2) (`self.previousSelection`))
              ;[1 1 1] Change the previous lane to be open(false) now
              (`KismetArrayLibrary.Array_Set` (`self.Lanes`) (`self.previousSelection`))
              ;[1 1 1] Move actor over
              (`self.ShiftLaneOfShot` (`self.SelectedShot`) (`self.Left`) self)
              ;[1 1 1] If an actor is in new lane->true else
              (if (`KismetArrayLibrary.Array_Get` (`self.Lanes`) (`self.pickedLane`))
                (if (not (== (`self.SelectedShot`) null))
                  ;[1 0.01209 0] Loop through all shots to find the one in the new lane
                  (bind _outactors_2 (`GameplayStatics.GetAllActorsOfClass` "/Game/Blueprints/shot.shot_C"))
                  (for _array_element_2 _outactors_2
                    (bind _asshot_c_2 (cast `/Game/Blueprints/shot` _array_element_2))
                    (if (== (`/Game/Blueprints/shot.Lane` _asshot_c_2) (`self.pickedLane`))
                      (set `self.newLaneShot` _asshot_c_2)))
                  ;[1 0.03055 0] Make sure the selected shot is from the new lane
                  (if (== (`/Game/Blueprints/shot.Lane` (`self.newLaneShot`)) (`self.pickedLane`))
                    ;[1 1 1] delay then destroy both actors
                    (`KismetSystemLibrary.Delay` 0.5)
                    (`self.destroyboth` _selectedshot _newlaneshot (+ (`/Game/Blueprints/shot.Damage` _newlaneshot) (`/Game/Blueprints/shot.Damage` _selectedshot)) (`KismetMathLibrary.MakeTransform` (`KismetMathLibrary.VLerp` (.location (`self.GetTransform` (`self.SelectedShot`))) (.location (`self.GetTransform` (`self.newLaneShot`))) 0.5) (.rotation (`self.GetTransform`)) (1.0 1.0 1.0)) (`self.pickedLane`) self)))
                (else
                  (set `/Game/Blueprints/shot.Lane` (`self.pickedLane`) (`self.SelectedShot`))
                  (`KismetArrayLibrary.Array_Set` (`self.Lanes`) (`self.pickedLane`) true))))))
        (set `self.previousSelection` -1))
      (:`==`
        (if (`KismetArrayLibrary.Array_Get` (`self.Lanes`) (`self.pickedLane`))
          ;[1 1 1] double check if open lanes is open
          (`self.checkOpenLanes`)
          (if (`KismetArrayLibrary.Array_Get` (`self.Lanes`) (`self.pickedLane`))
            (set `self.previousSelection` (`self.pickedLane`))
            (else
              (`KismetArrayLibrary.Array_Set` (`self.Lanes`) (`self.pickedLane`) true :!label _label_2)
              (bind _transform (`self.getShotLocation`))
              (`self.shot` _transform (`self.pickedLane`) (`self.PlayerId`) self)))
          (else
            (goto _label_2)))))))

(event `Key|Two`
  (:`Pressed`
    (set `self.pickedLane` 1)
    (set `self.distanceMultiplier` 0.0)
    (goto _label)))

(event `Key|Three`
  (bind _returnvalue (== (`self.PlayerId`) 0))
  (:`Pressed`
    (set `self.pickedLane` (`KismetMathLibrary.SelectInt` 2 0 _returnvalue))
    (set `self.distanceMultiplier` (`KismetMathLibrary.SelectFloat` 1.0 -1.0 _returnvalue))
    (goto _label)))

(event `shot`
  (params (transform :type "Object.Transform Structure") (lane :type Integer) (playerId :type Integer) (NewParam :type "Object Object Reference"))
  (bind _returnvalue (`|SpawnActorFromClass` "/Game/Blueprints/shot.shot_C" transform true))
  (set `/Game/Blueprints/shot.Player` playerId _returnvalue)
  (set `/Game/Blueprints/shot.Lane` lane _returnvalue)
  (set `/Game/Blueprints/shot.playerObject` NewParam _returnvalue))

(event `self.Box1.OnComponentBeginOverlap`
  (params (OtherActor :type "Actor Object Reference") (OtherComp :type "PrimitiveComponent Object Reference") (OtherBodyIndex :type Integer))
  ;[1 1 1] PlayerTakeDamage
  (bind _asshot_c (cast `/Game/Blueprints/shot` OtherActor))
  (if (!= (`/Game/Blueprints/shot.Player` _asshot_c) -1)
    (bind _asshot_c_2 (cast `/Game/Blueprints/shot` _asshot_c))
    (bind _playerobject (`/Game/Blueprints/shot.playerObject` _asshot_c_2))
    (if (!= _playerobject self)
      (bind _asplayerpawn_c (cast `/Game/Blueprints/playerPawn` _playerobject))
      (set `/Game/Blueprints/playerPawn.shotsFired` false _asplayerpawn_c)
      (bind _lane (`/Game/Blueprints/shot.Lane` _asshot_c))
      (`KismetArrayLibrary.Array_Set` (`/Game/Blueprints/playerPawn.Lanes` _asplayerpawn_c) _lane)
      (if (== _lane (`/Game/Blueprints/playerPawn.previousSelection` _asplayerpawn_c))
        (set `/Game/Blueprints/playerPawn.previousSelection` -1 _asplayerpawn_c))
      (`self.playerTakeDamage` 0 0 _asshot_c self))))

(event `playerTakeDamage`
  (params (playerId :type Integer) (Damage :type Integer) (object :type "Object Object Reference") (playerObject :type "Object Object Reference"))
  ;[1 1 1] PlayerTakeDamage
  (bind _asshot_c (cast `/Game/Blueprints/shot` object))
  (if (!= (`/Game/Blueprints/shot.playerObject` _asshot_c) playerObject)
    (bind _asplayerpawn_c (cast `/Game/Blueprints/playerPawn` playerObject))
    (set `/Game/Blueprints/playerPawn.health` (- (`/Game/Blueprints/playerPawn.health` _asplayerpawn_c) (`/Game/Blueprints/shot.Damage` _asshot_c)) _asplayerpawn_c)
    (`GameplayStatics.PlaySoundAtLocation` "/Game/Audio/Collapse01.Collapse01")
    (`self.K2_DestroyActor` _asshot_c)))

(fn `checkOpenLanes`
  (for _index (range 7)
    (`KismetArrayLibrary.Array_Set` (`self.Lanes`) _index))
  (bind _outactors (`GameplayStatics.GetAllActorsOfClass` "/Game/Blueprints/shot.shot_C"))
  (for _array_element _outactors
    (bind _asshot_c (cast `/Game/Blueprints/shot` _array_element))
    (if (== (`/Game/Blueprints/shot.playerObject` _asshot_c) self)
      (`KismetArrayLibrary.Array_Set` (`self.Lanes`) (`/Game/Blueprints/shot.Lane` _asshot_c) true))))

(fn `getShotLocation`
  (returns (transform :type "Object.Transform Structure"))
  (return (`KismetMathLibrary.MakeTransform` (`KismetMathLibrary.MakeVector` (.x (.location (`self.GetTransform`))) (+ (* (`self.distanceMultiplier`) 100.0) (.y (.location (`self.GetTransform`)))) (.z (.location (`self.GetTransform`)))) (.rotation (`self.GetTransform`)))))

(fn `OnRep_SelectedShot`)

(fn `UserConstructionScript`)